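; Actor that rides a referenced spline track and damages idea_of_circle actors it overlaps.
; If active at BeginPlay, a timeline drives its location and rotation along the spline, with configurable duration and start offset.
; On overlap, it increments the circle's damage count, shrinks its sphere and calls ChangeSize, using a DoOnce with delayed reset as a cooldown.
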(event `self.ReceiveBeginPlay`
  ;[1 1 1] movement
  (if (`self.activeMent`)
    (`self.Move`)))

(event `self.ReceiveActorBeginOverlap`
  (params (OtherActor :type "Actor Object Reference"))
  ;[1 1 1] change size of circle
  (bind _asidea_of_circle (cast `/Game/Blueprints/idea_of_circle` OtherActor))
  (`/Engine/EditorBlueprintResources/StandardMacros.DoOnce` false :!label _label
    (:`Completed`
      (set `/Game/Blueprints/idea_of_circle.how_much_damage` (+ (`/Game/Blueprints/idea_of_circle.how_much_damage` _asidea_of_circle) 1) _asidea_of_circle)
      (bind _sphere (`/Game/Blueprints/idea_of_circle.Sphere` _asidea_of_circle))
      (`SceneComponent.SetRelativeScale3D` _sphere (- (`SceneComponent.RelativeScale3D` _sphere) (0.2 0.2 0.2)))
      (`/Game/Blueprints/idea_of_circle.change size` _asidea_of_circle)
      (`KismetSystemLibrary.Delay` 3.0)
      (goto _label :!via `Reset`))))

(event `Move`
  (bind _returnvalue (`KismetMathLibrary.Lerp` 0.0 (`SplineComponent.GetSplineLength` (`/Game/Blueprints/track.UsefulSpline` (`self.TrackRef`))) (`self.Alpha`)))
  ;[1 1 1] movement
  (`TimelineComponent.SetPlayRate` (`self.Mover`) (/ 1.0 (`self.Duration`)))
  (`TimelineComponent.SetNewTime` (`self.Mover`) (`self.CartStartOffset`))
  (bind (_direction _alpha) (`Timeline|Mover`)
    (:`Update`
      (set `self.Alpha` _alpha)
      (`self.K2_SetActorLocationAndRotation` (`SplineComponent.GetLocationAtDistanceAlongSpline` (`/Game/Blueprints/track.UsefulSpline` (`self.TrackRef`)) _returnvalue "World") (`SplineComponent.GetRotationAtDistanceAlongSpline` (`/Game/Blueprints/track.UsefulSpline` (`self.TrackRef`)) _returnvalue "Local")))))

(fn `UserConstructionScript`)