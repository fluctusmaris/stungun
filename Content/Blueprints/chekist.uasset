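; Chekist is a hazard actor that can patrol along a referenced track's spline and kills the idea_of_circle actor on contact.
; On BeginPlay a timeline animates the cube's emissive strength, and if ActiveMent is set, Move starts the Mover timeline.
; Mover, scaled by Duration and starting at CartStartOffset, maps alpha to spline distance, using world location but local rotation.
; Overlap plays a death sound, then calls Death on the circle after a short delay.
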(event `self.ReceiveBeginPlay`
  ;[1 1 1] movement
  (`|ExecutionSequence`
    (:`then_0`
      (bind (_direction _glowwwwwwww) (`Timeline|glow chekist glow`)
        (:`Update`
          (`MeshComponent.SetScalarParameterValueOnMaterials` (`self.Cube`) "Emissive Strength" _glowwwwwwww))))
    (:`then_1`
      (if (`self.activeMent`)
        (`self.Move`)))))

(event `Move`
  (bind _returnvalue (`KismetMathLibrary.Lerp` 0.0 (`SplineComponent.GetSplineLength` (`/Game/Blueprints/track.UsefulSpline` (`self.TrackRef`))) (`self.Alpha`)))
  ;[1 1 1] movement
  (`TimelineComponent.SetPlayRate` (`self.Mover`) (/ 1.0 (`self.Duration`)))
  (`TimelineComponent.SetNewTime` (`self.Mover`) (`self.CartStartOffset`))
  (bind (_direction _alpha) (`Timeline|Mover`)
    (:`Update`
      (set `self.Alpha` _alpha)
      (`self.K2_SetActorLocationAndRotation` (`SplineComponent.GetLocationAtDistanceAlongSpline` (`/Game/Blueprints/track.UsefulSpline` (`self.TrackRef`)) _returnvalue "World") (`SplineComponent.GetRotationAtDistanceAlongSpline` (`/Game/Blueprints/track.UsefulSpline` (`self.TrackRef`)) _returnvalue "Local")))))

(event `self.ReceiveActorBeginOverlap`
  (params (OtherActor :type "Actor Object Reference"))
  ;[1 1 1] death of circle
  (bind _asidea_of_circle (cast `/Game/Blueprints/idea_of_circle` OtherActor))
  (`GameplayStatics.PlaySound2D` "/Game/sounds/chekist_die_Cue.chekist_die_Cue" 1.0 1.0 0.0 null null)
  (`KismetSystemLibrary.Delay` 0.2)
  (`/Game/Blueprints/idea_of_circle.death` _asidea_of_circle))

(fn `UserConstructionScript`)