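; Player character for the circle "idea", moved in fixed steps by touch swipes, that counts picked-up ideas.
; Externally set damage drives changesize, which swaps the sphere's material and lengthens steps, though the third hit only sets the size variable.
; The fourth hit triggers death: collision off, a timeline burn effect that creates the lose menu every update, then an idea-count reset.
; It also handles pausing through a reused menu widget.
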(event `death`
  (bind _returnvalue (`GameplayStatics.GetPlayerController` 0))
  ;[1 1 1] death
  (`PrimitiveComponent.SetCollisionEnabled` (`self.CapsuleComponent`) "NoCollision")
  (`PrimitiveComponent.SetCollisionEnabled` (`self.Mesh`) "NoCollision")
  (`PrimitiveComponent.SetMaterial` (`self.Sphere`) 0 "/Game/material/idea_picked_up.idea_picked_up")
  (bind (_direction _zagorelsya_krugov_dom) (`Timeline|delay krasivo`)
    (:`Update`
      (`MeshComponent.SetScalarParameterValueOnMaterials` (`self.Sphere`) "Burn" _zagorelsya_krugov_dom)
      (bind _returnvalue_2 (`|CreateWidget` "/Game/ui/widgets/lose_menu.lose_menu_C" _returnvalue))
      (`UserWidget.AddToViewport` _returnvalue_2 0)
      (`WidgetBlueprintLibrary.SetInputMode_UIOnlyEx` _returnvalue _returnvalue_2))
    (:`Finished`
      (set `self.pickedup_ideas` 0))))

(event `change size`
  ;[1 1 1] change size
  (if (== (`self.how_much_damage`) 4)
    (`self.death`)
    (elif (== (`self.how_much_damage`) 1)
      (set `self.which_size` "NewEnumerator1")
      (switch `/Game/Blueprints/size_of_circle` (`self.which_size`) :!label _label
        (:`NewEnumerator0`
          (`PrimitiveComponent.SetMaterial` (`self.Sphere`) 0 "/Game/material/idea_of_circle_1.idea_of_circle_1")
          (set `self.movement_points` 50.0))
        (:`NewEnumerator1`
          (`PrimitiveComponent.SetMaterial` (`self.Sphere`) 0 "/Game/material/idea_of_circle_07.idea_of_circle_07")
          (set `self.movement_points` 75.0))
        (:`NewEnumerator2`
          (`PrimitiveComponent.SetMaterial` (`self.Sphere`) 0 "/Game/material/idea_of_circle_04.idea_of_circle_04")
          (set `self.movement_points` 100.0))
        (:`NewEnumerator3`
          (`PrimitiveComponent.SetMaterial` (`self.Sphere`) 0 "/Game/material/idea_of_circle_01.idea_of_circle_01")
          (set `self.movement_points` 125.0)))
      (elif (== (`self.how_much_damage`) 2)
        (set `self.which_size` "NewEnumerator2")
        (goto _label)
        (elif (== (`self.how_much_damage`) 3)
          (set `self.which_size` "NewEnumerator3"))))))

(event `InputAction|Pause`
  (params (Key :type "Key Structure"))
  ;[1 1 1] Pause Game
  (:`Pressed`
    (`self.PauseGame`)))

(event `got_idea`
  ;[1 1 1] ideas
  (set `self.pickedup_ideas` (+ (`self.pickedup_ideas`) 1)))

(event `InputTouch`
  (params (Location :type "Vector Structure") (FingerIndex :type "ETouchIndex Enum"))
  (bind _x (.x (- (`self.currentTouchLocation`) (`self.startTouchLocation`))))
  (bind _y (.y (- (`self.currentTouchLocation`) (`self.startTouchLocation`))))
  ;[1 1 1] swipe movement
  (:`Pressed`
    (set `self.startTouchLocation` Location)
    (set `self.isSwiping?` true))
  (:`Moved`
    (set `self.currentTouchLocation` Location)
    (if (`self.isSwiping?`)
      (if (> (`KismetMathLibrary.VSize` (- (`self.currentTouchLocation`) (`self.startTouchLocation`))) 100.0)
        (set `self.isSwiping?` false)
        (if (> (`KismetMathLibrary.Abs` _x) (`KismetMathLibrary.Abs` _y))
          (if (> _x 0.0)
            (`self.K2_AddActorLocalOffset` (`KismetMathLibrary.MakeVector` 0.0 (`self.movement_points`)))
            (else
              (`self.K2_AddActorLocalOffset` (`KismetMathLibrary.MakeVector` 0.0 (* -1 (`self.movement_points`))))))
          (elif (> _y 0.0)
            (`self.K2_AddActorLocalOffset` (`KismetMathLibrary.MakeVector` (* -1 (`self.movement_points`))))
            (else
              (`self.K2_AddActorLocalOffset` (`KismetMathLibrary.MakeVector` (`self.movement_points`))))))))))

(fn `PauseGame`
  (`GameplayStatics.SetGamePaused` true)
  (`/Engine/EditorBlueprintResources/StandardMacros.IsValid` (`self.PauseMenu`)
    (:`Is Valid`
      _)
    (:`Is Not Valid`
      (bind _returnvalue (`|CreateWidget` "/Game/ui/widgets/pause_menu_widget.pause_menu_widget_C" (`GameplayStatics.GetPlayerController` 0)))
      (set `self.PauseMenu` _returnvalue)))
  (`UserWidget.AddToViewport` (`self.PauseMenu`) 0)
  (`WidgetBlueprintLibrary.SetInputMode_UIOnlyEx` (`GameplayStatics.GetPlayerController` 0) (`self.PauseMenu`))
  (set `PlayerController.bShowMouseCursor` true (`GameplayStatics.GetPlayerController` 0)))

(fn `UnpauseGame`
  (bind _returnvalue (`GameplayStatics.GetPlayerController` 0))
  (`GameplayStatics.SetGamePaused` false)
  (`Widget.RemoveFromParent` (`self.PauseMenu`))
  (`WidgetBlueprintLibrary.SetInputMode_GameOnly` _returnvalue)
  (set `PlayerController.bShowMouseCursor` true _returnvalue))

(fn `UserConstructionScript`)