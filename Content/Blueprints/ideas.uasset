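; An idea pickup actor that spins its plane and is collected when an idea_of_circle actor overlaps it.
; On BeginPlay, a timeline drives the plane's yaw.
; On overlap it plays a sound, swaps to the picked-up material and animates its Burn scalar through a second timeline.
; When that timeline finishes, it calls GotIdea on the overlapping actor and destroys itself.
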(event `self.ReceiveActorBeginOverlap`
  (params (OtherActor :type "Actor Object Reference"))
  ;[1 1 1] pick up
  (bind _asidea_of_circle (cast `/Game/Blueprints/idea_of_circle` OtherActor))
  (`GameplayStatics.PlaySound2D` "/Game/sounds/pickup_idea_Cue.pickup_idea_Cue" 1.0 1.0 0.0 null null)
  (`PrimitiveComponent.SetMaterial` (`self.Plane`) 0 "/Game/material/idea_picked_up.idea_picked_up")
  (bind (_direction _burn_baby_burn) (`Timeline|delau_kruto`)
    (:`Update`
      (`MeshComponent.SetScalarParameterValueOnMaterials` (`self.Plane`) "Burn" _burn_baby_burn))
    (:`Finished`
      (`/Game/Blueprints/idea_of_circle.got_idea` _asidea_of_circle)
      (`self.K2_DestroyActor`))))

(event `self.ReceiveBeginPlay`
  ;[1 1 1] movement attraction
  (bind (_direction _rotation) (`Timeline|something nice`)
    (:`Update`
      (`SceneComponent.K2_SetRelativeRotation` (`self.Plane`) (`KismetMathLibrary.MakeRotator` 0.0 0.0 _rotation) false false))))

(fn `UserConstructionScript`)